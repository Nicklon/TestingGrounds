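; BP_Tile is one segment of an infinite terrain, scattering cubes and AI enemy pawns on BeginPlay.
; A Lock trigger opens the barrier (green, no collision) while the player overlaps it, reporting the tile conquered once to InfiniteTerrainGamemode, and closes it (red) on exit.
; A DestroyTile trigger asks the game mode to spawn another tile, then destroys this one.
; An arrow supplies the attach transform, and a FirstLevel flag starts the barrier open.
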(event `self.ReceiveBeginPlay`
  (if (`self.FirstLevel`)
    (`self.LockDisabled`))
  (`self.PlaceActors` "/Game/Dynamic/Terrain/Props/BP_Cube.BP_Cube_C" 1 20 80.0 1.0 5.0)
  (`self.PlaceAIPawns` "/Game/Dynamic/Character/Behaviour/BP_Character.BP_Character_C" (`self.MinEnemies`) (`self.MaxEnemies`) 100.0))

(event `self.Lock.OnComponentBeginOverlap`
  (params (OverlappedComponent :type "PrimitiveComponent Object Reference") (OtherActor :type "Actor Object Reference") (OtherComp :type "PrimitiveComponent Object Reference") (OtherBodyIndex :type Integer) (bFromSweep :type Boolean) (SweepResult :type "HitResult Structure (by ref)"))
  (`self.IsPlayer` OtherActor
    (:`True`
      (`|ExecutionSequence`
        (:`then_0`
          (`self.LockDisabled`))
        (:`then_1`
          (`self.TileConquered`))))))

(event `self.Lock.OnComponentEndOverlap`
  (params (OverlappedComponent :type "PrimitiveComponent Object Reference") (OtherActor :type "Actor Object Reference") (OtherComp :type "PrimitiveComponent Object Reference") (OtherBodyIndex :type Integer))
  (`self.IsPlayer` OtherActor
    (:`True`
      (`self.LockEnabled`))))

(event `self.DestroyTile.OnComponentBeginOverlap`
  (params (OverlappedComponent :type "PrimitiveComponent Object Reference") (OtherActor :type "Actor Object Reference") (OtherComp :type "PrimitiveComponent Object Reference") (OtherBodyIndex :type Integer) (bFromSweep :type Boolean) (SweepResult :type "HitResult Structure (by ref)"))
  (`self.IsPlayer` OtherActor
    (:`True`
      (bind _asinfinite_terrain_gamemode (cast `/Game/Dynamic/InfiniteTerrainGamemode` (`GameplayStatics.GetGameMode`)))
      (`/Game/Dynamic/InfiniteTerrainGamemode.Spawn Tile` _asinfinite_terrain_gamemode)
      (`self.K2_DestroyActor`))))

(fn `Get Attach Location`
  (returns (`Attach Transform` :type "Transform Structure"))
  (return (`SceneComponent.K2_GetComponentToWorld` (`self.Arrow`))))

(fn `LockDisabled`
  (bind _barrier (`self.Barrier`))
  (`PrimitiveComponent.SetCollisionEnabled` _barrier "NoCollision")
  (`PrimitiveComponent.SetMaterial` _barrier 0 "/Game/Static/Geometry/Materials/MI_Barrier_Green.MI_Barrier_Green"))

(fn `LockEnabled`
  (bind _barrier (`self.Barrier`))
  (`PrimitiveComponent.SetCollisionEnabled` _barrier "QueryAndPhysics")
  (`PrimitiveComponent.SetMaterial` _barrier 0 "/Game/Static/Geometry/Materials/MI_Barrier_Red.MI_Barrier_Red"))

(fn `TileConquered`
  (if (not (`self.IsTileConquered`))
    (bind _asinfinite_terrain_gamemode (cast `/Game/Dynamic/InfiniteTerrainGamemode` (`GameplayStatics.GetGameMode`)))
    (`/Game/Dynamic/InfiniteTerrainGamemode.NewTileConquered` _asinfinite_terrain_gamemode)
    (set `self.IsTileConquered` true)))

(fn `UserConstructionScript`)